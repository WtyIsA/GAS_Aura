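; Enemy melee attack gameplay ability that turns the avatar toward its combat target and plays a random tagged attack montage.
; The montage's gameplay event triggers a small sphere query at the matching combat socket, damaging non-friendly live players and calling their blood effect.
; Any hit fires one melee impact GameplayCue carrying the montage tag.
; The ability ends after the hit check or when the montage completes or is interrupted.
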(event Ability|EventActivateAbility
  (bind _returnvalue (Ability|GetAvatarActorfromActorInfo))
  (bind _returnvalue_2 (Ability|GetAvatarActorfromActorInfo))
  (bind _returnvalue_3 (Ability|GetAvatarActorfromActorInfo))
  (Variables|Default|SetHasHitTarget false)
  (bind _returnvalue_4 (Class|EnemyInterface|GetCombatTarget(Message) _returnvalue_3))
  (bind _ascombat_interface (Utilities|Casting|CastToCombatInterface _returnvalue_3))
  (Class|CombatInterface|UpdateFacingTarget _ascombat_interface (Transformation|GetActorLocation _returnvalue_4))
  (bind _returnvalue_5 (Class|CombatInterface|GetAttackMontages(Message) _returnvalue_3))
  (bind _output_get (Variables|Default|SetTaggedMontage (Class|AuraDamageGameplayAbility|GetRandomTaggedMontagefromArray _returnvalue_5)))
  (|PlayMontageandWaitProxy "None" (.montage _output_get) 1.0 "None" false 1.0 0.0 false
    (:then
      (Ability|Tasks|WaitGameplayEvent (.montagetag _output_get) 0
        (:EventReceived
          (bind _returnvalue_6 (Class|CombatInterface|GetCombatSocketLocation(Message) _returnvalue (.sockettag _output_get)))
          (Variables|Default|SetCombatSocketLocation _returnvalue_6)
          (bind _outoverlappingactors (Class|AuraAbilitySystemLibrary|GetLivePlayerswithRadius _returnvalue (Utilities|Array|MakeArray _returnvalue) 45.0 (Variables|Default|GetCombatSocketLocation)))
          (for _array_element _outoverlappingactors
            (if (Class|AuraAbilitySystemLibrary|IsNotFriend (Ability|GetAvatarActorfromActorInfo) _array_element)
              (Class|AuraDamageGameplayAbility|CauseDamage _array_element)
              (Variables|Default|SetHasHitTarget true)
              (Class|CombatInterface|GetBloodEffect(Message) _array_element)))
          (if (Variables|Default|GetHasHitTarget)
            (bind _returnvalue_7 (Class|EnemyInterface|GetCombatTarget(Message) _returnvalue_2))
            (Class|GameplayAbility|ExecuteGameplayCuewithParams "(TagName=\"GameplayCue.MeleeImpact\")" (Ability|GameplayCue|MakeGameplayCueParameters :AggregatedSourceTags (GameplayTags|MakeGameplayTagContainerfromTag (.MontageTag (Utilities|Struct|BreakTaggedMontage (Variables|Default|GetTaggedMontage)))) :Location (Variables|Default|GetCombatSocketLocation) :EffectCauser _returnvalue_2 :SourceObject _returnvalue_7)))
          (Ability|EndAbility))))
    (:OnCompleted
      (Ability|EndAbility :!label _label))
    (:OnInterrupted
      (goto _label))
    (:OnCancelled
      (goto _label))))

(event Ability|EventOnEndAbility
  (params (bWasCancelled :type Boolean)))